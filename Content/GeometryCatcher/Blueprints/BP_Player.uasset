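; BP_Player is the player pawn in GeometryCatcher, moving sideways along its right axis and handling game pause.
; The MoveRight axis feeds movement input scaled by MaxSpeed along the actor's right vector.
; Tick consumes that vector and applies it as a delta-time-scaled, swept local offset, moving the pawn directly without a movement component.
; The P key toggles game pause through the IsPaused flag.
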(event `self.ReceiveBeginPlay`)

(event `Key|P` :paused true
  (params (Key :type "Key Structure"))
  ;[1 1 1] Пауза на P, при повторном нажатии продолжение игры
  (:`Pressed`
    (if (`self.IsPaused`)
      (set `self.IsPaused` false)
      (`GameplayStatics.SetGamePaused` false)
      (else
        (set `self.IsPaused` true)
        (`GameplayStatics.SetGamePaused` true)))))

(event `self.ReceiveTick`
  (params (DeltaSeconds :type "Float (single-precision)"))
  (bind _returnvalue (`self.ConsumeMovementInputVector`))
  (`self.K2_AddActorLocalOffset` (* _returnvalue DeltaSeconds) true))

(event `InputAxis|MoveRight`
  (params (AxisValue :type "Float (single-precision)"))
  (`self.AddMovementInput` (`self.GetActorRightVector`) (* AxisValue (`self.MaxSpeed`))))

(fn `UserConstructionScript`)